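; Title screen game mode that handles the title music and the key that moves the game between title, playing and game over states.
; On BeginPlay it enables input and plays the looping main theme only if MyGameInstance reports the title state.
; Pressing Z on the title fades out the playing theme, waits for the fade, then sets the state to playing.
; Pressing Z during game over sets the state back to title.
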(event `self.ReceiveBeginPlay`
  (bind _main_theme05_loop (`self.main-theme05_loop`))
  (bind _asmy_game_instance (cast `MyGameInstance` (`GameplayStatics.GetGameInstance`)))
  (if (`|EnumEquality` (`MyGameInstance.GetCurrentState` _asmy_game_instance) "ETitle")
    (`AudioComponent.Play` _main_theme05_loop 0.0)
    (else
      (`AudioComponent.Stop` _main_theme05_loop)))
  (`self.EnableInput` (`GameplayStatics.GetPlayerController` 0)))

(event `Key|Z`
  (params (Key :type "Key Structure"))
  (bind _main_theme05_loop (`self.main-theme05_loop`))
  (:`Pressed`
    (bind _asmy_game_instance (cast `MyGameInstance` (`GameplayStatics.GetGameInstance`)))
    (if (`|EnumEquality` (`MyGameInstance.GetCurrentState` _asmy_game_instance) "ETitle")
      (if (`AudioComponent.IsPlaying` _main_theme05_loop)
        (`AudioComponent.FadeOut` _main_theme05_loop 2.0 0.0 "Linear")
        (`KismetSystemLibrary.Delay` 2.0)
        (bind _asmy_game_instance_2 (cast `MyGameInstance` (`GameplayStatics.GetGameInstance`)))
        (`MyGameInstance.SetCurrentState` _asmy_game_instance_2 "EPlaying"))
      (else
        (bind _asmy_game_instance_3 (cast `MyGameInstance` (`GameplayStatics.GetGameInstance`)))
        (if (`|EnumEquality` (`MyGameInstance.GetCurrentState` _asmy_game_instance_3) "EGameOver")
          (bind _asmy_game_instance_4 (cast `MyGameInstance` (`GameplayStatics.GetGameInstance`)))
          (`MyGameInstance.SetCurrentState` _asmy_game_instance_4 "ETitle"))))))

(fn `UserConstructionScript`)