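; Player character Blueprint with modular body and gear meshes and unfinished enemy highlighting.
; BeginPlay slaves the face, hair and gear meshes to the main Mesh through master pose.
; Tick rebinds an empty overlap handler on components inside EnemyCollisionVolume, checks and stores its SweepResult as Enemy, and passes HighlightActor to Trace.
; Trace enables custom depth on the actor's "Outline"-tagged skeletal mesh; a forward sphere trace is left unwired.
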(event `self.ReceiveBeginPlay`
  (`SkinnedMeshComponent.SetLeaderPoseComponent` (`self.Face`) (`self.Mesh`) false)
  (`SkinnedMeshComponent.SetLeaderPoseComponent` (`self.Hair`) (`self.Mesh`) false)
  (`SkinnedMeshComponent.SetLeaderPoseComponent` (`self.Gloves`) (`self.Mesh`) false)
  (`SkinnedMeshComponent.SetLeaderPoseComponent` (`self.Shoes`) (`self.Mesh`) false)
  (`SkinnedMeshComponent.SetLeaderPoseComponent` (`self.HeadGears`) (`self.Mesh`) false)
  (`SkinnedMeshComponent.SetLeaderPoseComponent` (`self.ShoulderPad`) (`self.Mesh`) false)
  (`SkinnedMeshComponent.SetLeaderPoseComponent` (`self.Belt`) (`self.Mesh`) false))

(event `self.ReceiveTick`
  (params (DeltaSeconds :type "Float (single-precision)"))
  (add `PrimitiveComponent.OnComponentBeginOverlap` (`PrimitiveComponent.GetOverlappingComponents` (`self.EnemyCollisionVolume`)) (delegate `OnComponentBeginOverlap_Event_0`))
  (if (not (== (`.HitActor` (`GameplayStatics.BreakHitResult` (stale `OnComponentBeginOverlap_Event_0` SweepResult))) null))
    (`self.Trace` (`|GetArrayItem` (`self.HighlightActor`) 1)))
  (set `self.Enemy` (stale `OnComponentBeginOverlap_Event_0` SweepResult)))

(event `OnActorBeginOverlap_Event_0`
  (params (OverlappedActor :type "Actor Object Reference") (OtherActor :type "Actor Object Reference")))

(event `OnComponentBeginOverlap_Event_0`
  (params (OverlappedComponent :type "PrimitiveComponent Object Reference") (OtherActor :type "Actor Object Reference") (OtherComp :type "PrimitiveComponent Object Reference") (OtherBodyIndex :type Integer) (bFromSweep :type Boolean) (SweepResult :type "HitResult Structure (by ref)")))

(fn `Trace`
  (params (NewActor :type "Actor Object Reference"))
  (`PrimitiveComponent.SetRenderCustomDepth` (`|GetArrayItem` (`self.GetComponentsByTag` NewActor "/Script/Engine.SkeletalMeshComponent" "Outline")) true))

(fn `UserConstructionScript`)